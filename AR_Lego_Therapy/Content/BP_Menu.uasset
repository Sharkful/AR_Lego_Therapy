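; BP_Menu is a hand-attached menu actor for role selection, built on UX Tools palm-up constraint.
; It starts in a Selection state and, while in that state, shows RoleSelectionMenu when the palm-up constraint activates and hides it when it deactivates.
; Pressing the Builder button switches the state to Confirmation, after which the palm gesture no longer toggles the selection menu; no Confirmation behavior is implemented yet.
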(event OnConstraintActivated(UxtPalmUpConstraint)
  (switch string (Variables|Default|GetState)
    (:Selection
      (Class|UxtUIElementComponent|SetUIVisibility (Variables|Default|GetRole%20Selection%20Menu) "Show"))))

(event OnConstraintDeactivated(UxtPalmUpConstraint)
  (switch string (Variables|Default|GetState)
    (:Selection
      (Class|UxtUIElementComponent|SetUIVisibility (Variables|Default|GetRole%20Selection%20Menu) "Hide"))))

(event OnComponentActivated(BuilderButton)
  (params (Component :type Actor%20Component%20Object%20Reference) (bReset :type Boolean))
  (Variables|Default|SetState "Confirmation"))

(event EventBeginPlay
  (Variables|Default|SetState "Selection"))

(event Collision|EventActorBeginOverlap
  (params (OtherActor :type Actor%20Object%20Reference)))

(event EventTick
  (params (DeltaSeconds :type Float%20%28single-precision%29)))

(fn ConstructionScript)